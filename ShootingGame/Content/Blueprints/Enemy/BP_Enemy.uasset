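; Pooled enemy character that loads stats by Type from the GameInstance data table and takes its target from the AI blackboard.
; Looping timers drive melee or pooled-bullet attacks on the player and healing of other enemies.
; Damage updates a health widget; death grants EXP, spawns pooled drops and returns the enemy to its pool.
; Effect events handle stun, slow and area damage; DoT hits the player instantly, and knockback is unwired.
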(event `Heal`
  (bind (_returnvalue_roll _returnvalue_pitch _returnvalue_yaw) (`KismetMathLibrary.BreakRotator` (`KismetMathLibrary.FindLookAtRotation` (`self.K2_GetActorLocation`) (`self.K2_GetActorLocation` (`self.TargetActor`)))))
  (bind _returnvalue (`KismetSystemLibrary.K2_SetTimerDelegate` (delegate `Heal`) 0.5 true))
  (set `self.HealTimer` _returnvalue)
  (`self.K2_SetActorRotation` (`KismetMathLibrary.MakeRotator` 0.0 0.0 _returnvalue_yaw))
  (bind _asbp_enemy (cast `/Game/Blueprints/Enemy/BP_Enemy` (`self.TargetActor`)))
  (`self.GetHeal` _asbp_enemy (`self.HealAmount`)))

(event `self.ReceiveBeginPlay`
  (bind _healthcomponent (`self.HealthComponent`))
  (bind _asbp_game_instance (cast `/Game/Blueprints/BP_GameInstance` (`GameplayStatics.GetGameInstance`)))
  (set `self.Game Instance` _asbp_game_instance)
  (for _array_element (`/Game/Blueprints/DA/BP_EnemyDataTable.EnemyDatas` (`/Game/Blueprints/BP_GameInstance.EnemyDataTable` (`self.Game Instance`)))
    (if (`|EnumEquality` (`self.Type`) (`.Type_17_DFBC38FC40B4E945393EF2A3FA997185` (break `/Game/Blueprints/ST/ST_EnemyData` _array_element)))
      (set `self.Damage` (break `/Game/Blueprints/ST/ST_EnemyData` _array_element))
      (set `self.ShootForce` (`.ShootForce_29_179DB68C4F49232DF43D6985F28A8F7C` (break `/Game/Blueprints/ST/ST_EnemyData` _array_element)))
      (set `self.AttackRange` (`.AttackRange_9_CB88E80B4249A798EA04D3B00FE61545` (break `/Game/Blueprints/ST/ST_EnemyData` _array_element)))
      (set `self.AttackType` (`.AttackType_11_E2444DA9497795B9F1FDA3BF1D3AEA9C` (break `/Game/Blueprints/ST/ST_EnemyData` _array_element)))
      (set `self.Bullet Effects` (`.EnemyEffects_50_459C58764FADEF45EEFEB1866CE336C3` (break `/Game/Blueprints/ST/ST_EnemyData` _array_element)))
      (set `self.Exp` (`.Exp_36_96B609F64E8E298427A3D4B424DFCC4D` (break `/Game/Blueprints/ST/ST_EnemyData` _array_element)))
      (set `/Game/Blueprints/AC/AC_Health.MaxHealth` (`.Health_39_A9199AFF470722C56E9B3FAE2128B549` (break `/Game/Blueprints/ST/ST_EnemyData` _array_element)) _healthcomponent)
      (set `/Game/Blueprints/AC/AC_Health.CurrentHealth` (`.Health_39_A9199AFF470722C56E9B3FAE2128B549` (break `/Game/Blueprints/ST/ST_EnemyData` _array_element)) _healthcomponent)
      (set `self.HealAmount` (`.HealAmount_55_598552B64E11E8DEA387539C6D62B52E` (break `/Game/Blueprints/ST/ST_EnemyData` _array_element)))
      (bind _aswbp_enemy_health (cast `/Game/Blueprints/Enemy/WBP_EnemyHealth` (`WidgetComponent.GetUserWidgetObject` (`self.Widget`))))
      (set `self.WBP Enemy Health` _aswbp_enemy_health)
      (bind _asbp_player (cast `/Game/Blueprints/Player/BP_Player` (`GameplayStatics.GetPlayerPawn` 0)))
      (set `self.Player` _asbp_player))))

(event `Attack`
  (bind _returnvalue (`SceneComponent.K2_GetComponentLocation` (`self.Muzzle`)))
  (bind (_returnvalue_roll _returnvalue_pitch _returnvalue_yaw) (`KismetMathLibrary.BreakRotator` (`KismetMathLibrary.FindLookAtRotation` (`self.K2_GetActorLocation`) (`self.K2_GetActorLocation` (`self.TargetActor`)))))
  (bind _returnvalue_2 (`KismetSystemLibrary.K2_SetTimerDelegate` (delegate `Attack`) 0.5 true))
  (set `self.AttackTimer` _returnvalue_2)
  (if (not (`/Game/Blueprints/Player/BP_Player.IsDead` (`self.Player`)))
    (`self.K2_SetActorRotation` (`KismetMathLibrary.MakeRotator` 0.0 0.0 _returnvalue_yaw))
    (switch `/Game/Blueprints/EState/Estate_EnemyAttack` (`self.AttackType`)
      (:`NewEnumerator0`
        ; 근거리 공격
        (`/Game/Blueprints/Player/BP_Player.GetDamage` (`self.Player`) (`self.Damage`))
        (for _array_element (`self.Bullet Effects`)
          (`/Game/Blueprints/BPI/BPI_BulletEffect.ApplyEffect` _array_element (`self.Player`) 1.0)))
      (:`NewEnumerator1`
        ; 원거리 공격
        (bind _bullet (`/Game/Blueprints/BP_PoolManager.GetEnemyBullet` (`/Game/Blueprints/BP_GameInstance.PoolManager` (`self.Game Instance`)) (`self.Type`)))
        (`self.K2_SetActorLocation` _bullet _returnvalue false true)
        (`/Game/Blueprints/Enemy/BP_EnemyBullet.ActivateBullet` _bullet (* (`KismetMathLibrary.Normal` (- (`SceneComponent.K2_GetComponentLocation` (`Character.CapsuleComponent` (`GameplayStatics.GetPlayerCharacter` 0))) _returnvalue)) (`self.ShootForce`)) _returnvalue (`self.Damage`) (`self.Bullet Effects`))))))

(event `self.ReceiveTick`
  (params (DeltaSeconds :type "Float (single-precision)"))
  (bind (_returnvalue_roll _returnvalue_pitch _returnvalue_yaw) (`KismetMathLibrary.BreakRotator` (`KismetMathLibrary.FindLookAtRotation` (`self.K2_GetActorLocation`) (`self.K2_GetActorLocation` (`GameplayStatics.GetPlayerPawn` 0)))))
  (`self.K2_SetActorRotation` (`KismetMathLibrary.MakeRotator` 0.0 0.0 _returnvalue_yaw))
  (bind `_as액터` (cast `Actor` (`BlackboardComponent.GetValueAsObject` (`AIBlueprintHelperLibrary.GetBlackboard` (`AIBlueprintHelperLibrary.GetAIController` (`self.GetController`))) (`self.TargetActorName`))))
  (set `self.TargetActor` `_as액터`))

(event `GetHeal`
  (params (Val :type "Float (double-precision)"))
  (bind _healthcomponent (`self.HealthComponent`))
  (if (`self.IsActive`)
    (`/Game/Blueprints/AC/AC_Health.GetHeal` (`self.HealthComponent`) Val)
    (set `/Game/Blueprints/Enemy/WBP_EnemyHealth.TargetHpPercent` (/ (`/Game/Blueprints/AC/AC_Health.CurrentHealth` _healthcomponent) (`/Game/Blueprints/AC/AC_Health.MaxHealth` _healthcomponent)) (`self.WBP Enemy Health`))))

(event `GetDamage`
  (params (Val :type "Float (double-precision)"))
  (bind _healthcomponent (`self.HealthComponent`))
  (bind _healthcomponent_2 (`self.HealthComponent`))
  (bind _returnvalue (`KismetMathLibrary.RandomPointInBoundingBox` (`self.K2_GetActorLocation`) (100.0 100.0 0.0)))
  (if (`self.IsActive`)
    (`/Game/Blueprints/AC/AC_Health.GetDamage` _healthcomponent Val)
    (set `/Game/Blueprints/Enemy/WBP_EnemyHealth.TargetHpPercent` (/ (`/Game/Blueprints/AC/AC_Health.CurrentHealth` _healthcomponent_2) (`/Game/Blueprints/AC/AC_Health.MaxHealth` _healthcomponent_2)) (`self.WBP Enemy Health`))
    ; Die
    (if (<= (`/Game/Blueprints/AC/AC_Health.CurrentHealth` _healthcomponent) 0.0)
      (bind _asbp_enemy_aicontroller (cast `/Game/Blueprints/Enemy/AI/BP_EnemyAIController` (`self.GetController`)))
      (`BrainComponent.StopLogic` (`AIController.BrainComponent` _asbp_enemy_aicontroller) "")
      (set `self.AnimSpeed` 3.0)
      (`KismetSystemLibrary.Delay` 1.0)
      (`/Game/Blueprints/Player/BP_Player.UpdateExp` (`self.Player`) (`self.Exp`))
      (bind _newparam (`/Game/Blueprints/BP_GameInstance.FindEnemyDropData` (`self.Game Instance`) (`self.Type`)))
      (for _array_element _newparam
        (if (`|EnumEquality` (break `/Game/Blueprints/ST/ST_EnemyDropItem` _array_element) "NewEnumerator0")
          (for _ (range 1 (+ (/ (`.Num_5_4A5BF56344E68D464485EA83486D976F` (break `/Game/Blueprints/ST/ST_EnemyDropItem` _array_element)) 10) 1))
            (bind _upgitem (`/Game/Blueprints/BP_PoolManager.GetUpgItem` (`/Game/Blueprints/BP_GameInstance.PoolManager` (`self.Game Instance`)) (break `/Game/Blueprints/ST/ST_EnemyDropItem` _array_element)))
            (`/Game/Blueprints/Item/BP_Item.Activate` _upgitem _returnvalue))
          (else
            (for _ (range 1 (+ (`.Num_5_4A5BF56344E68D464485EA83486D976F` (break `/Game/Blueprints/ST/ST_EnemyDropItem` _array_element)) 1))
              (bind _upgitem_2 (`/Game/Blueprints/BP_PoolManager.GetUpgItem` (`/Game/Blueprints/BP_GameInstance.PoolManager` (`self.Game Instance`)) (break `/Game/Blueprints/ST/ST_EnemyDropItem` _array_element)))
              (`/Game/Blueprints/Item/BP_Item.Activate` _upgitem_2 _returnvalue)))))
      (`self.DeActivateEnemy`)
      (`/Game/Blueprints/ObjectPool.Return` (`self.ParentPool`) self))))

(event `GetAnimVal`
  (params (Val :type "Float (double-precision)"))
  (set `self.AnimSpeed` Val))

(event `DeActivateEnemy`
  ; 비활성화
  (`self.K2_SetActorLocation` (0.0 0.0 0.0))
  (`ActorComponent.SetActive` (`self.Mesh`) false false)
  (`self.SetActorHiddenInGame` true)
  (bind _asbp_enemy_aicontroller (cast `/Game/Blueprints/Enemy/AI/BP_EnemyAIController` (`self.GetController`)))
  (`BrainComponent.StopLogic` (`AIController.BrainComponent` _asbp_enemy_aicontroller) "")
  (set `self.IsActive` false))

(event `StopAttack`
  (`KismetSystemLibrary.K2_ClearAndInvalidateTimerHandle` (`self.AttackTimer`)))

(event `StopHeal`
  (`KismetSystemLibrary.K2_ClearAndInvalidateTimerHandle` (`self.HealTimer`)))

(event `ActivateEnemy`
  (params (SpawnPos :type "Vector Structure"))
  (bind _healthcomponent (`self.HealthComponent`))
  (bind _healthcomponent_2 (`self.HealthComponent`))
  ; 활성화
  (`self.K2_SetActorLocation` SpawnPos)
  (bind _asbp_enemy_aicontroller (cast `/Game/Blueprints/Enemy/AI/BP_EnemyAIController` (`self.GetController`)))
  (`BrainComponent.RestartLogic` (`AIController.BrainComponent` _asbp_enemy_aicontroller))
  (`ActorComponent.SetActive` (`self.Mesh`) true false)
  (`self.SetActorHiddenInGame` false)
  (set `self.AnimSpeed` 0.0)
  (set `/Game/Blueprints/AC/AC_Health.CurrentHealth` (`/Game/Blueprints/AC/AC_Health.MaxHealth` _healthcomponent) _healthcomponent)
  (set `/Game/Blueprints/Enemy/WBP_EnemyHealth.TargetHpPercent` (/ (`/Game/Blueprints/AC/AC_Health.CurrentHealth` _healthcomponent_2) (`/Game/Blueprints/AC/AC_Health.MaxHealth` _healthcomponent_2)) (`self.WBP Enemy Health`))
  (set `self.IsActive` true))

(event `/Game/Blueprints/BPI/BPI_BulletEffectReceiver.ApplyStun`
  (params (StunTime :type "Float (double-precision)"))
  (bind _charactermovement (`self.CharacterMovement`))
  ; 이펙트 적용
  ;; Stun
  (if (not (`self.IsStunned`))
    (set `self.IsStunned` true)
    (bind _output_get (set `self.OriSpeed` (`CharacterMovementComponent.MaxWalkSpeed` _charactermovement)))
    (set `CharacterMovementComponent.MaxWalkSpeed` 0.0 _charactermovement)
    (`KismetSystemLibrary.Delay` 0.2)
    (set `CharacterMovementComponent.MaxWalkSpeed` _output_get _charactermovement)
    (set `self.IsStunned` false)))

(event `/Game/Blueprints/BPI/BPI_BulletEffectReceiver.ApplySlow`
  (params (SlowAmount :type "Float (double-precision)") (SlowTime :type "Float (double-precision)"))
  (bind _charactermovement (`self.CharacterMovement`))
  ; 이펙트 적용
  ;; Slow
  (if (not (`self.IsSlowed`))
    (set `self.IsSlowed` true)
    (set `CharacterMovementComponent.MaxWalkSpeed` (* (`CharacterMovementComponent.MaxWalkSpeed` _charactermovement) SlowAmount) _charactermovement)
    (`KismetSystemLibrary.Delay` SlowTime)
    (set `CharacterMovementComponent.MaxWalkSpeed` (/ (`CharacterMovementComponent.MaxWalkSpeed` _charactermovement) SlowAmount) _charactermovement)
    (set `self.IsSlowed` false)))

(event `/Game/Blueprints/BPI/BPI_BulletEffectReceiver.ApplyDotdam`
  (params (DotDamage :type "Float (double-precision)") (DotNum :type Integer))
  ; 이펙트 적용
  ;; Dotdam
  (for _ (range (+ DotNum 1))
    (`/Game/Blueprints/AC/AC_Health.GetDamage` (`/Game/Blueprints/Player/BP_Player.HealthComponent` (`self.Player`)) DotDamage)))

(event `/Game/Blueprints/BPI/BPI_BulletEffectReceiver.ApplyRange`
  (params (Radius :type "Float (double-precision)") (RangeDam :type "Float (double-precision)"))
  ; 이펙트 적용
  (bind _outactors (`KismetSystemLibrary.SphereOverlapActors` (`SceneComponent.K2_GetComponentLocation` (`self.CapsuleComponent`)) Radius (`self.Object Types_0`) "BP_Enemy_C"))
  (for _array_element _outactors
    (bind _asbp_enemy (cast `/Game/Blueprints/Enemy/BP_Enemy` _array_element))
    (`self.GetDamage` _asbp_enemy RangeDam)))

(event `/Game/Blueprints/BPI/BPI_BulletEffectReceiver.ApplyKnockback`
  (params (Force :type "Float (double-precision)") (Radius :type "Float (double-precision)")))

(fn `UserConstructionScript`)