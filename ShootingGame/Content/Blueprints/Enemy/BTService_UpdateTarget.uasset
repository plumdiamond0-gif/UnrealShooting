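; Behavior tree service that refreshes an enemy's target and attack state on the blackboard for BP_Enemy pawns.
; On each AI tick it sets the player character as the target and writes the distance between the enemy and the player.
; It sets the CanAttack flag by comparing that distance against the enemy's AttackRange.
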(event `self.ReceiveTickAI`
  (params (OwnerController :type "AIController Object Reference") (ControlledPawn :type "Pawn Object Reference") (DeltaSeconds :type "Float (single-precision)"))
  (bind _returnvalue (`GameplayStatics.GetPlayerCharacter` 0))
  (bind _returnvalue_2 (`KismetMathLibrary.Vector_Distance` (`Actor.K2_GetActorLocation` ControlledPawn) (`Actor.K2_GetActorLocation` _returnvalue)))
  (bind _asbp_enemy (cast `/Game/Blueprints/Enemy/BP_Enemy` ControlledPawn))
  (`BTFunctionLibrary.SetBlackboardValueAsObject` (`self.TargetActorKey`) _returnvalue)
  (`BTFunctionLibrary.SetBlackboardValueAsFloat` (`self.Diatance`) _returnvalue_2)
  (if (< _returnvalue_2 (`/Game/Blueprints/Enemy/BP_Enemy.AttackRange` _asbp_enemy))
    (`BTFunctionLibrary.SetBlackboardValueAsBool` (`self.CanAttack`) true)
    (else
      (`BTFunctionLibrary.SetBlackboardValueAsBool` (`self.CanAttack`)))))