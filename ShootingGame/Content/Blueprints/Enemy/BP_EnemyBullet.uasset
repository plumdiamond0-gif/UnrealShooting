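; BP_EnemyBullet is a pooled enemy projectile that damages BP_Player on sphere overlap and applies its effects.
; ActivateBullet sets velocity, damage, effects and origin, while DeActivateBullet hides it and disables collision and movement.
; A player hit deactivates it and re-adds it to ParentPool inside the effect loop, once per effect.
; The max-distance recycle on Tick is switched off by a constant false condition.
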(event `self.ReceiveTick`
  (params (DeltaSeconds :type "Float (single-precision)"))
  (bind _parentpool (`self.ParentPool`))
  (if (and (> (`KismetMathLibrary.Vector_Distance` (`self.OriPos`) (`self.K2_GetActorLocation`)) (`self.MaxDist`)) false)
    (`self.DeActivateBullet`)
    (set `MovementComponent.Velocity` (0.0 0.0 0.0) (`self.ProjectileMovement`))
    (`/Engine/EditorBlueprintResources/StandardMacros.IsValid` _parentpool
      (:`Is Valid`
        (`KismetArrayLibrary.Array_Add` (`/Game/Blueprints/ObjectPool.PoolObjects` _parentpool) self)))))

(event `DeActivateBullet`
  ; 탄환 비활성화
  (`PrimitiveComponent.SetCollisionEnabled` (`self.Sphere`) "NoCollision")
  (`ActorComponent.SetActive` (`self.ProjectileMovement`) false false)
  (`self.SetActorHiddenInGame` true)
  (set `MovementComponent.Velocity` (0.0 0.0 0.0) (`self.ProjectileMovement`)))

(event `ActivateBullet`
  (params (Velocity :type "Vector Structure") (Pos :type "Vector Structure") (FinalDamage :type "Float (double-precision)") (Effects :type "Array of /Game/Blueprints/DA/Effect/BP_BulletEffect Object Reference"))
  ; 탄환 활성화
  (`PrimitiveComponent.SetCollisionEnabled` (`self.Sphere`) "QueryOnly")
  (set `self.Effects` Effects)
  (set `self.Damage` FinalDamage)
  (`ActorComponent.SetActive` (`self.ProjectileMovement`) true false)
  (set `self.OriPos` Pos)
  (`self.SetActorHiddenInGame` false)
  (set `MovementComponent.Velocity` Velocity (`self.ProjectileMovement`)))

(event `self.Sphere.OnComponentBeginOverlap`
  (params (OverlappedComponent :type "PrimitiveComponent Object Reference") (OtherActor :type "Actor Object Reference") (OtherComp :type "PrimitiveComponent Object Reference") (OtherBodyIndex :type Integer) (bFromSweep :type Boolean) (SweepResult :type "HitResult Structure (by ref)"))
  (bind _parentpool (`self.ParentPool`))
  ; 플레이아에게 닿았을 시
  (bind _asbp_player (cast `/Game/Blueprints/Player/BP_Player` OtherActor))
  (`/Game/Blueprints/Player/BP_Player.GetDamage` _asbp_player (`self.Damage`))
  (`self.DeActivateBullet`)
  (for _array_element (`self.Effects`)
    (`/Game/Blueprints/BPI/BPI_BulletEffect.ApplyEffect` _array_element _asbp_player 1.0)
    (`/Engine/EditorBlueprintResources/StandardMacros.IsValid` _parentpool
      (:`Is Valid`
        (`KismetArrayLibrary.Array_Add` (`/Game/Blueprints/ObjectPool.PoolObjects` _parentpool) self)))))

(fn `UserConstructionScript`)