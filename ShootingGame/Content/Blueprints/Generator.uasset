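; Spawner actor that produces enemies, in-game items or inventory items, chosen by its GenerateType, while the player is nearby.
; Tick compares player distance to DetectRange, starting a self-rescheduling 60-second timer on entry and clearing it on exit.
; Enemies come from the GameInstance pool at random nearby points; items spawn by type from GameInstance data tables.
; Inventory items respawn only when the last spawned one is collected or invalid.
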(event `self.ReceiveBeginPlay`
  (cast `/Game/Blueprints/BP_GameMode` (`GameplayStatics.GetGameMode`))
  (bind _asbp_game_instance (cast `/Game/Blueprints/BP_GameInstance` (`GameplayStatics.GetGameInstance`)))
  (set `self.BP Game Instance` _asbp_game_instance)
  (bind _asbp_player (cast `/Game/Blueprints/Player/BP_Player` (`GameplayStatics.GetPlayerPawn` 0)))
  (set `self.Player` _asbp_player))

(event `GenerateObject`
  (bind (_returnvalue_x _returnvalue_y) (`KismetMathLibrary.BreakVector` (`self.K2_GetActorLocation`)))
  (bind (_returnvalue_x_2 _returnvalue_y_2) (`KismetMathLibrary.BreakVector` (`self.K2_GetActorLocation`)))
  (bind _bp_game_instance (`self.BP Game Instance`))
  (bind _spawneditem (`self.SpawnedItem`))
  (bind (_returnvalue_x_3 _returnvalue_y_3 _returnvalue_z) (`KismetMathLibrary.BreakVector` (`KismetMathLibrary.RandomPointInBoundingBox` (`self.K2_GetActorLocation`) (300.0 300.0 0.0))))
  (bind _returnvalue (`KismetSystemLibrary.K2_SetTimerDelegate` (delegate `GenerateObject`) 60.0))
  (set `self.GenerateTimer` _returnvalue)
  (switch `/Game/Blueprints/EState/EState_Generate` (`self.GenerateType`)
    (:`NewEnumerator0`
      ; Enemy
      (for _ (range 1 (+ (`self.GenerateNum`) 1))
        (bind _enemy (`/Game/Blueprints/BP_PoolManager.GetEnmey` (`/Game/Blueprints/BP_GameInstance.PoolManager` _bp_game_instance) (`self.EnemyType`)))
        (`/Engine/EditorBlueprintResources/StandardMacros.IsValid` _enemy
          (:`Is Valid`
            (`/Game/Blueprints/Enemy/BP_Enemy.ActivateEnemy` _enemy (`KismetMathLibrary.MakeVector` _returnvalue_x_3 _returnvalue_y_3 (+ _returnvalue_z 85.0)))))))
    (:`NewEnumerator1`
      ; InItem
      (for _ (range 1 (+ (`self.GenerateNum`) 1))
        (for _array_element (`/Game/Blueprints/DA/BP_InItemDataTable.InItemDatas` (`/Game/Blueprints/BP_GameInstance.InItemDataTable` _bp_game_instance))
          (if (`|EnumEquality` (`.InItemType_23_0EFB35C64F4033E0B1E3B1A45CE1999A` (break `/Game/Blueprints/ST/ST_InItemData` _array_element)) (`self.InItemType`))
            (bind _returnvalue_2 (`|SpawnActorFromClass` (`.ItemClass_25_A19311204F4E8E334D02169CA945F7D3` (break `/Game/Blueprints/ST/ST_InItemData` _array_element)) (`KismetMathLibrary.MakeTransform` (0.0 0.0 30.0)) "AlwaysSpawn" "MultiplyWithRoot" null null))
            (bind _output_get (set `self.SpawnedItem` _returnvalue_2))
            (`/Game/Blueprints/Item/BP_Item.Activate` _output_get (`KismetMathLibrary.MakeVector` _returnvalue_x_2 _returnvalue_y_2 0.0))))))
    (:`NewEnumerator2`
      (`/Engine/EditorBlueprintResources/StandardMacros.IsValid` _spawneditem
        (:`Is Valid`
          (if (`/Game/Blueprints/Item/BP_Item.IsCollected` _spawneditem)
            ; InvUtem
            (for _ (range 1 (+ (`self.GenerateNum`) 1)) :!label _label
              (for _array_element_2 (`/Game/Blueprints/DA/BP_InvItemDataTable.InvItemDatas` (`/Game/Blueprints/BP_GameInstance.InvItemDataTable` _bp_game_instance))
                (if (`|EnumEquality` (`.Type_5_DE5CCAEF4AAF58300EB0FD96F0C0CBC6` (break `/Game/Blueprints/ST/ST_InvItemData` _array_element_2)) (`self.InvItemType`))
                  (bind _returnvalue_3 (`|SpawnActorFromClass` (`.Class_11_BC60E2754766E787FAFB689DDAAFD367` (break `/Game/Blueprints/ST/ST_InvItemData` _array_element_2)) (`KismetMathLibrary.MakeTransform` (0.0 0.0 30.0)) "AlwaysSpawn" "MultiplyWithRoot" null null))
                  (bind _output_get_2 (set `self.SpawnedItem` _returnvalue_3))
                  (`/Game/Blueprints/Item/BP_Item.Activate` _output_get_2 (`KismetMathLibrary.MakeVector` _returnvalue_x _returnvalue_y 30.0)))))))
        (:`Is Not Valid`
          (goto _label))))))

(event `StopGenerate`
  (`KismetSystemLibrary.K2_ClearAndInvalidateTimerHandle` (`self.GenerateTimer`)))

(event `self.ReceiveTick`
  (params (DeltaSeconds :type "Float (single-precision)"))
  (if (< (`KismetMathLibrary.Vector_Distance` (`self.K2_GetActorLocation` (`self.Player`)) (`self.K2_GetActorLocation`)) (`self.DetectRange`))
    (if (not (`self.IsGenerate`))
      (`self.GenerateObject`)
      (set `self.IsGenerate` true))
    (elif (`self.IsGenerate`)
      (`self.StopGenerate`)
      (set `self.IsGenerate` false))))

(fn `UserConstructionScript`)