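; AC_Health is a component that tracks current health and a temporary invincibility state for its owner.
; GetDamage subtracts from CurrentHealth unless invincible, and GetHeal adds to it, both without clamping or death handling in the graph.
; BeInvincible sets the invincibility flag, waits for the given time with a Delay, then clears it.
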(event `BeInvincible`
  (params (time :type "Float (double-precision)"))
  (set `self.IsInvincible` true)
  (`KismetSystemLibrary.Delay` time)
  (set `self.IsInvincible` false))

(event `GetDamage`
  (params (Damage :type "Float (double-precision)"))
  (if (not (`self.IsInvincible`))
    (set `self.CurrentHealth` (- (`self.CurrentHealth`) Damage))))

(event `GetHeal`
  (params (Heal :type "Float (double-precision)"))
  (set `self.CurrentHealth` (+ (`self.CurrentHealth`) Heal)))