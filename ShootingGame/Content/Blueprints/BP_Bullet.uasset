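; BP_Bullet is a reusable projectile actor that damages BP_Enemy targets, toggled on and off instead of destroyed.
; ActivateBullet stores damage and origin, shows the bullet and sets its ProjectileMovement velocity.
; Tick hides and stops it once it travels beyond MaxDist from that origin.
; A Sphere overlap with a BP_Enemy applies damage through its HealthComponent, then hides the bullet and deactivates its movement.
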(event `self.ReceiveBeginPlay`)

(event `self.ReceiveTick`
  (params (DeltaSeconds :type "Float (single-precision)"))
  (if (and (> (`KismetMathLibrary.Vector_Distance` (`self.OriPos`) (`self.K2_GetActorLocation`)) (`self.MaxDist`)) (`self.IsUsing`))
    (`self.SetActorHiddenInGame` true)
    (set `MovementComponent.Velocity` (0.0 0.0 0.0) (`self.ProjectileMovement`))
    (set `self.IsUsing` false)))

(event `DeActivateBullet`
  ; 탄환 비활성화
  (`ActorComponent.SetActive` (`self.ProjectileMovement`) false false)
  (`self.SetActorHiddenInGame` true))

(event `ActivateBullet`
  (params (Velocity :type "Vector Structure") (Pos :type "Vector Structure") (FinalDamage :type "Float (double-precision)"))
  ; 탄환 활성화
  (set `self.Damage` FinalDamage)
  (`ActorComponent.SetActive` (`self.ProjectileMovement`) true false)
  (set `self.OriPos` Pos)
  (`self.SetActorHiddenInGame` false)
  (set `MovementComponent.Velocity` Velocity (`self.ProjectileMovement`))
  (set `self.IsUsing` true))

(event `self.Sphere.OnComponentBeginOverlap`
  (params (OverlappedComponent :type "PrimitiveComponent Object Reference") (OtherActor :type "Actor Object Reference") (OtherComp :type "PrimitiveComponent Object Reference") (OtherBodyIndex :type Integer) (bFromSweep :type Boolean) (SweepResult :type "HitResult Structure (by ref)"))
  ; 플레이어에게 닿았을 시
  (bind _asbp_enemy (cast `/Game/Blueprints/Enemy/BP_Enemy` OtherActor))
  (`/Game/Blueprints/HealthComponent.GetDamage` (`/Game/Blueprints/Enemy/BP_Enemy.HealthComponent` _asbp_enemy) (`self.Damage`))
  (`self.SetActorHiddenInGame` true)
  (set `MovementComponent.Velocity` (0.0 0.0 0.0) (`self.ProjectileMovement`))
  (set `self.IsUsing` false)
  (`self.DeActivateBullet`))

(fn `UserConstructionScript`)