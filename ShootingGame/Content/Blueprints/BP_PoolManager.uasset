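; BP_PoolManager pre-spawns and serves pooled player bullets, enemies and enemy bullets by type.
; On BeginPlay it reads enemy and bullet data from the BP_GameInstance tables and builds an ObjectPool per entry, keyed by type in three maps.
; Each pooled actor gets a ParentPool back-reference and starts deactivated.
; Getter functions look up the pool by type and return a cast actor from it.
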(event `self.ReceiveBeginPlay`
  (bind _asbp_game_instance (cast `/Game/Blueprints/BP_GameInstance` (`GameplayStatics.GetGameInstance`)))
  (set `self.Bullet Datas` (`/Game/Blueprints/DA/BP_BulletTable/BP_BulletDataTable.BulletDatas` (`/Game/Blueprints/BP_GameInstance.BulletDataTable` _asbp_game_instance)))
  (set `self.Enemy Datas` (`/Game/Blueprints/DA/BP_EnemyDataTable.EnemyDatas` (`/Game/Blueprints/BP_GameInstance.EnemyDataTable` _asbp_game_instance)))
  (`|ExecutionSequence`
    (:`then_0`
      ; 탄환 생성
      (for _array_element (`self.Enemy Datas`)
        (bind _returnvalue (`|SpawnActorFromClass` "/Game/Blueprints/ObjectPool.ObjectPool_C" (`KismetMathLibrary.MakeTransform` (0.0 0.0 0.0)) "Undefined" "MultiplyWithRoot" null null))
        (bind (_damage _attackrange _attacktype _name _type _bp_class _spawnnum) (break `/Game/Blueprints/ST/ST_EnemyData` _array_element))
        (`/Game/Blueprints/ObjectPool.Initialize` _returnvalue _bp_class _spawnnum)
        (`BlueprintMapLibrary.Map_Add` (`self.EnemyPool`) _type _returnvalue)
        (for _array_element_2 (`/Game/Blueprints/ObjectPool.PoolObjects` _returnvalue)
          (bind _asbp_enemy (cast `/Game/Blueprints/Enemy/BP_Enemy` _array_element_2))
          (set `/Game/Blueprints/Enemy/BP_Enemy.ParentPool` _returnvalue _asbp_enemy)
          (`/Game/Blueprints/Enemy/BP_Enemy.DeActivateEnemy` _asbp_enemy))))
    (:`then_1`
      (for _array_element_3 (`self.Bullet Datas`)
        (bind _returnvalue_2 (`|SpawnActorFromClass` "/Game/Blueprints/ObjectPool.ObjectPool_C" (`KismetMathLibrary.MakeTransform` (0.0 0.0 0.0)) "Undefined" "MultiplyWithRoot" null null))
        (bind (_damage_2 _shootingspeed _effects _bulletname _bullettype _recoilx _returnspeed _recoilyz _cancharge _actorclass _spawnnum_2) (break `/Game/Blueprints/ST/ST_BulletData` _array_element_3))
        (`/Game/Blueprints/ObjectPool.Initialize` _returnvalue_2 _actorclass _spawnnum_2)
        (`BlueprintMapLibrary.Map_Add` (`self.BulletPool`) _bullettype _returnvalue_2)
        (for _array_element_4 (`/Game/Blueprints/ObjectPool.PoolObjects` _returnvalue_2)
          (bind _asbp_bullet (cast `/Game/Blueprints/Player/Bullet/BP_Bullet` _array_element_4))
          (set `/Game/Blueprints/Player/Bullet/BP_Bullet.ParentPool` _returnvalue_2 _asbp_bullet)
          (`/Game/Blueprints/Player/Bullet/BP_Bullet.DeActivateBullet` _asbp_bullet))))
    (:`then_2`
      (for _array_element_5 (`self.Enemy Datas`)
        (bind _returnvalue_3 (`|SpawnActorFromClass` "/Game/Blueprints/ObjectPool.ObjectPool_C" (`KismetMathLibrary.MakeTransform` (0.0 0.0 0.0)) "AlwaysSpawn" "MultiplyWithRoot" null null))
        (bind (_damage_3 _attackrange_2 _attacktype_2 _name_2 _type_2 _bp_class_2 _spawnnum_3 _enemyeffects _shootforce _bulletspawncount _exp _health _bulletclass) (break `/Game/Blueprints/ST/ST_EnemyData` _array_element_5))
        (`/Game/Blueprints/ObjectPool.Initialize` _returnvalue_3 _bulletclass _bulletspawncount)
        (`BlueprintMapLibrary.Map_Add` (`self.EnemyBulletPool`) _type_2 _returnvalue_3)
        (for _array_element_6 (`/Game/Blueprints/ObjectPool.PoolObjects` _returnvalue_3)
          (bind _asbp_enemy_bullet (cast `/Game/Blueprints/Enemy/BP_EnemyBullet` _array_element_6))
          (set `/Game/Blueprints/Enemy/BP_EnemyBullet.ParentPool` _returnvalue_3 _asbp_enemy_bullet)
          (`/Game/Blueprints/Enemy/BP_EnemyBullet.DeActivateBullet` _asbp_enemy_bullet))))))

(fn `GetBullet`
  (params (Type :type "/Game/Blueprints/EState/EState_Bullet Enum" :default "NewEnumerator5"))
  (returns (Bullet :type "/Game/Blueprints/Player/Bullet/BP_Bullet Object Reference"))
  (bind _obj (`/Game/Blueprints/ObjectPool.Get` (`BlueprintMapLibrary.Map_Find` (`self.BulletPool`) Type)))
  (bind _asbp_bullet (cast `/Game/Blueprints/Player/Bullet/BP_Bullet` _obj))
  (return _asbp_bullet))

(fn `GetEnemyBullet`
  (params (Type :type "/Game/Blueprints/EState/EState_Enemy Enum" :default "NewEnumerator0"))
  (returns (Bullet :type "/Game/Blueprints/Enemy/BP_EnemyBullet Object Reference"))
  (bind _obj (`/Game/Blueprints/ObjectPool.Get` (`BlueprintMapLibrary.Map_Find` (`self.EnemyBulletPool`) Type)))
  (bind _asbp_enemy_bullet (cast `/Game/Blueprints/Enemy/BP_EnemyBullet` _obj))
  (return _asbp_enemy_bullet))

(fn `GetEnmey`
  (params (NewParam :type "/Game/Blueprints/EState/EState_Enemy Enum" :default "NewEnumerator0"))
  (returns (Enemy :type "/Game/Blueprints/Enemy/BP_Enemy Object Reference"))
  (bind _value (`BlueprintMapLibrary.Map_Find` (`self.EnemyPool`) NewParam))
  (bind _obj (`/Game/Blueprints/ObjectPool.Get` _value))
  (bind _asbp_enemy (cast `/Game/Blueprints/Enemy/BP_Enemy` _obj))
  (set `/Game/Blueprints/Enemy/BP_Enemy.ParentPool` _value _asbp_enemy)
  (return _asbp_enemy))

(fn `UserConstructionScript`)