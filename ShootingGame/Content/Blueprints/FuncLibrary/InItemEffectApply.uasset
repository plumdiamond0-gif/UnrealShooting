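; Blueprint library function that applies a picked item type's buff to the player.
; It loops over the item data array for entries matching the given type, then switches on that type.
; Damage, attack speed and move speed multiply the player's current values, while health calls GetHeal.
; The attack speed buff scales PlayerShootForce, and move speed is written to the ACStat component.
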(fn `ItemEffectApply`
  (params (Player :type "/Game/Blueprints/Player/BP_Player Object Reference") (InItemType :type "/Game/Blueprints/EState/EState_BuffItem Enum" :default "NewEnumerator0") (InItrmDatas :type "Array of /Game/Blueprints/ST/ST_InItemData Structure"))
  (bind _ac_stat (`/Game/Blueprints/Player/BP_Player.AC_Stat` Player))
  (for _array_element InItrmDatas
    (if (`|EnumEquality` (`.InItemType_23_0EFB35C64F4033E0B1E3B1A45CE1999A` (break `/Game/Blueprints/ST/ST_InItemData` _array_element)) InItemType)
      (switch `/Game/Blueprints/EState/EState_BuffItem` InItemType
        (:`NewEnumerator0`
          ; DamageBuff
          (set `/Game/Blueprints/Player/BP_Player.PlayerDamage` (* (break `/Game/Blueprints/ST/ST_InItemData` _array_element) (`/Game/Blueprints/Player/BP_Player.PlayerDamage` Player)) Player)
          (break))
        (:`NewEnumerator1`
          ; Heal
          (`/Game/Blueprints/Player/BP_Player.GetHeal` Player (`.HealthBuff_12_131DCCC74D1F84BD5858A78281064D56` (break `/Game/Blueprints/ST/ST_InItemData` _array_element)))
          (break))
        (:`NewEnumerator2`
          ; AttackSpeedBuff
          (set `/Game/Blueprints/Player/BP_Player.PlayerShootForce` (* (`/Game/Blueprints/Player/BP_Player.PlayerShootForce` Player) (`.AttackSpeedBuff_10_641AACB14458A8BE5C94E69D24D604EE` (break `/Game/Blueprints/ST/ST_InItemData` _array_element))) Player)
          (break))
        (:`NewEnumerator3`
          ; MoveSpeedBuff
          (set `/Game/Blueprints/AC/AC_Stat.PlayerSpeed` (* (`.MoveSpeedBuff_9_5F0E8EA54CA79BA92216779AE85BE127` (break `/Game/Blueprints/ST/ST_InItemData` _array_element)) (`/Game/Blueprints/AC/AC_Stat.PlayerSpeed` _ac_stat)) _ac_stat))))))