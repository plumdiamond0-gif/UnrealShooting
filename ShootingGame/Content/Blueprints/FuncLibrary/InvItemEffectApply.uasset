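; Blueprint function library function that applies the effect of an inventory item, chosen by its type, to the player or enemies.
; It looks up duration and texture in the Game Instance's item data, then, for timed items, calls the player's item-use check and update dispatcher.
; A switch then deals heavy damage to a random half or so of active enemies, or triggers timed invincibility, recall beacon or berserker on the player.
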(fn `InvItemEffectApply`
  (params (Type :type "/Game/Blueprints/EState/EState_InvItem Enum" :default "NewEnumerator0") (WorldContextObject :type "Object Object Reference"))
  (locals (Texture :type "Texture2D Object Reference") (LastTime :type "Float (double-precision)"))
  (bind _lasttime (`local.LastTime`))
  (bind _asbp_game_instance (cast `/Game/Blueprints/BP_GameInstance` (`GameplayStatics.GetGameInstance` WorldContextObject)))
  (for _array_element (`/Game/Blueprints/DA/BP_InvItemDataTable.InvItemDatas` (`/Game/Blueprints/BP_GameInstance.InvItemDataTable` _asbp_game_instance))
    (bind (_texture _type _class _lastingtime) (break `/Game/Blueprints/ST/ST_InvItemData` _array_element))
    (if (`|EnumEquality` _type Type)
      (set `local.LastTime` _lastingtime)
      (set `local.Texture` _texture)
      (break)))
  (bind _asbp_player (cast `/Game/Blueprints/Player/BP_Player` (`GameplayStatics.GetPlayerCharacter` WorldContextObject)))
  (if (> _lasttime 0.0)
    (`/Game/Blueprints/Player/BP_Player.CanUseInvItem` _asbp_player (`local.LastTime`))
    (`/Game/Blueprints/Player/BP_Player.ED_UpdateInvItemUse` _asbp_player _lasttime (`local.Texture`) (`|GetEnumeratorNameAsString` _type)))
  (switch `/Game/Blueprints/EState/EState_InvItem` Type
    (:`NewEnumerator0`
      (bind _outactors (`GameplayStatics.GetAllActorsOfClass` WorldContextObject "/Game/Blueprints/Enemy/BP_Enemy.BP_Enemy_C"))
      (for _array_element_2 _outactors
        (if (and (`/Game/Blueprints/Enemy/BP_Enemy.IsActive` _array_element_2) (== (mod (`KismetMathLibrary.RandomInteger` 26) 2) 0))
          (`/Game/Blueprints/Enemy/BP_Enemy.GetDamage` _array_element_2 2600.0))))
    (:`NewEnumerator1`
      (`/Game/Blueprints/AC/AC_Health.BeInvincible` (`/Game/Blueprints/Player/BP_Player.HealthComponent` _asbp_player) (`local.LastTime`)))
    (:`NewEnumerator2`
      (`/Game/Blueprints/Player/BP_Player.RecallBeacon` _asbp_player (`local.LastTime`)))
    (:`NewEnumerator5`
      (`/Game/Blueprints/Player/BP_Player.Berserker` _asbp_player (`local.LastTime`)))))