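; BP_InvItem is an item actor that adds itself to a player's inventory when applied.
; On BeginPlay it looks up its texture by matching its Type against the InvItemDataTable held by the game instance.
; Apply fills the first empty inventory slot with the item type, fires the player's inventory update dispatcher with the texture and slot index, then deactivates the item.
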(event `self.ReceiveBeginPlay`
  (`parent.ReceiveBeginPlay`)
  (for _array_element (`/Game/Blueprints/DA/BP_InvItemDataTable.InvItemDatas` (`/Game/Blueprints/BP_GameInstance.InvItemDataTable` (`self.BP Game Instance`)))
    (if (`|EnumEquality` (`.Type_5_DE5CCAEF4AAF58300EB0FD96F0C0CBC6` (break `/Game/Blueprints/ST/ST_InvItemData` _array_element)) (`self.Type`))
      (set `self.Texture` (break `/Game/Blueprints/ST/ST_InvItemData` _array_element))
      (break))))

(fn `Apply`
  (params (Player :type "/Game/Blueprints/Player/BP_Player Object Reference"))
  (bind _inventory (`/Game/Blueprints/Player/BP_Player.Inventory` Player))
  (for (_array_element _array_index) _inventory
    (if (not (`.IsFilled_11_C5E600F944BFDB768DE7A09E481B8207` (break `/Game/Blueprints/ST/ST_InvSlot` _array_element)))
      (`KismetArrayLibrary.Array_Set` _inventory _array_index (make `/Game/Blueprints/ST/ST_InvSlot` (`self.Type`) true))
      (`/Game/Blueprints/Player/BP_Player.ED_UpdateInventoryGet` Player (`self.Texture`) _array_index)
      (`self.DeActivate`)
      (break))))

(fn `UserConstructionScript`
  (`parent.UserConstructionScript`))