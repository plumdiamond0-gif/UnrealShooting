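; Upgrade item pickup that homes in on the player and is added to their items on arrival.
; While active, Tick eases it toward player pawn 0 with VInterpTo.
; Mesh collision is disabled at BeginPlay, so pickup uses a distance check instead of overlap.
; Within range it passes its Type to the game instance's GetItem and calls DeActivate; the Apply function is empty.
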(event `self.ReceiveBeginPlay`
  (`PrimitiveComponent.SetCollisionEnabled` (`self.StaticMesh`) "NoCollision")
  (`parent.ReceiveBeginPlay`))

(event `self.ReceiveTick`
  (params (DeltaSeconds :type "Float (single-precision)"))
  (bind _returnvalue (`self.K2_GetActorLocation`))
  (bind _returnvalue_2 (`self.K2_GetActorLocation` (`GameplayStatics.GetPlayerPawn` 0)))
  (if (`self.IsActive`)
    (`self.K2_SetActorLocation` (`KismetMathLibrary.VInterpTo` _returnvalue _returnvalue_2 (`GameplayStatics.GetWorldDeltaSeconds`) 5.0))
    (`parent.ReceiveTick` DeltaSeconds)
    (if (< (`KismetMathLibrary.Vector_Distance` _returnvalue_2 _returnvalue) 100.0)
      (`/Game/Blueprints/BP_GameInstance.GetItem` (`self.BP Game Instance`) (`self.Type`) 1)
      (`self.DeActivate`))))

(fn `Apply`
  (params (Player :type "/Game/Blueprints/Player/BP_Player Object Reference")))

(fn `UserConstructionScript`
  (`parent.UserConstructionScript`))