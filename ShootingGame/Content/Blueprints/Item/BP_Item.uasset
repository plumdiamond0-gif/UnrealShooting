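; BP_Item is a rotating pickup actor that the player collects by touching it.
; On BeginPlay it caches the game instance and calls Activate; Activate and DeActivate toggle mesh collision and visibility.
; A mesh overlap with BP_Player calls Apply, an empty function here, then sets IsCollected.
; DeActivate is not called within this Blueprint, so collection alone does not hide the item.
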(event `self.ReceiveBeginPlay`
  (bind _asbp_game_instance (cast `/Game/Blueprints/BP_GameInstance` (`GameplayStatics.GetGameInstance`)))
  (set `self.BP Game Instance` _asbp_game_instance)
  (`self.Activate`))

(event `Activate`
  (`PrimitiveComponent.SetCollisionEnabled` (`self.StaticMesh`) "QueryOnly")
  (`self.SetActorHiddenInGame` false))

(event `self.ReceiveTick`
  (params (DeltaSeconds :type "Float (single-precision)"))
  (`SceneComponent.K2_AddWorldRotation` (`self.StaticMesh`) (struct :`Yaw` 2.0) false false))

(event `DeActivate`
  (`PrimitiveComponent.SetCollisionEnabled` (`self.StaticMesh`) "NoCollision")
  (`self.SetActorHiddenInGame` true))

(event `self.StaticMesh.OnComponentBeginOverlap`
  (params (OverlappedComponent :type "PrimitiveComponent Object Reference") (OtherActor :type "Actor Object Reference") (OtherComp :type "PrimitiveComponent Object Reference") (OtherBodyIndex :type Integer) (bFromSweep :type Boolean) (SweepResult :type "HitResult Structure (by ref)"))
  (bind _asbp_player (cast `/Game/Blueprints/Player/BP_Player` OtherActor))
  (`self.Apply` _asbp_player)
  (set `self.IsCollected` true))

(fn `Apply`
  (params (Player :type "/Game/Blueprints/Player/BP_Player Object Reference")))

(fn `UserConstructionScript`)