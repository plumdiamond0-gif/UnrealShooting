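; BP_KnockbackEffect is a bullet effect that applies knockback to a target actor.
; ApplyEffect scales the base Force and Radius by a factor interpolated between one and three, using the Multiplier as alpha.
; It then passes both scaled values to the target through the BPI_BulletEffectReceiver interface, and does nothing further if the target lacks it.
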(event `self.ApplyEffect`
  (params (TargetActor :type "Actor Object Reference") (Multiplier :type "Float (double-precision)"))
  (bind _returnvalue (`KismetMathLibrary.Lerp` 1.0 3.0 Multiplier))
  (`|ExecutionSequence`
    (:`then_0`
      (set `self.finalForce` (* (`self.Force`) _returnvalue))
      (set `self.finalRadius` (* (`self.Radius`) _returnvalue)))
    (:`then_1`
      (bind _asbpi_bullet_effect_receiver (cast `/Game/Blueprints/BulletEffects/BPI_BulletEffectReceiver` TargetActor))
      (`/Game/Blueprints/BulletEffects/BPI_BulletEffectReceiver.ApplyKnockback` _asbpi_bullet_effect_receiver (`self.finalForce`) (`self.finalRadius`)))))