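; Bullet effect Blueprint that applies a slow to the actor passed to its ApplyEffect event.
; The Multiplier blends a scale factor from 1 to 3, which divides the base slow amount and multiplies the base slow time.
; Both results go to ApplySlow through the BPI_BulletEffectReceiver interface, so targets without that interface receive no slow.
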(event `/Game/Blueprints/BulletEffects/BPI_BulletEffect.ApplyEffect`
  (params (TargetActor :type "Actor Object Reference") (Multiplier :type "Float (double-precision)"))
  (bind _returnvalue (`KismetMathLibrary.Lerp` 1.0 3.0 Multiplier))
  (`|ExecutionSequence`
    (:`then_0`
      (set `self.finalSlowAmount` (/ (`self.SlowAmount`) _returnvalue))
      (set `self.finalSlowTime` (* (`self.SlowTime`) _returnvalue)))
    (:`then_1`
      (bind _asbpi_bullet_effect_receiver (cast `/Game/Blueprints/BulletEffects/BPI_BulletEffectReceiver` TargetActor))
      (`/Game/Blueprints/BulletEffects/BPI_BulletEffectReceiver.ApplySlow` _asbpi_bullet_effect_receiver (`self.finalSlowAmount`) (`self.finalSlowTime`)))))