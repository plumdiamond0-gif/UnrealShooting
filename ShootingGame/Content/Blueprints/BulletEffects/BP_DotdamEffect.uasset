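; BP_DotdamEffect is a bullet effect that applies damage over time to a target actor.
; Its custom event scales the base damage and tick count by a Lerp between fixed bounds, using the incoming Multiplier as alpha, and truncates the count to an integer.
; It then casts the target to BPI_BulletEffectReceiver and passes both values to ApplyDotdam, leaving the damage handling to the receiver.
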(event `CustomEvent`
  (params (TargetActor :type "Actor Object Reference") (Multiplier :type "Float (double-precision)"))
  (bind _returnvalue (`KismetMathLibrary.Lerp` 1.0 3.0 Multiplier))
  (`|ExecutionSequence`
    (:`then_0`
      (set `self.finalDotNum` (`KismetMathLibrary.FTrunc` (* (`self.DotNum`) _returnvalue)))
      (set `self.finalDotdamage` (* (`self.DotDmaage`) _returnvalue)))
    (:`then_1`
      (bind _asbpi_bullet_effect_receiver (cast `/Game/Blueprints/BulletEffects/BPI_BulletEffectReceiver` TargetActor))
      (`/Game/Blueprints/BulletEffects/BPI_BulletEffectReceiver.ApplyDotdam` _asbpi_bullet_effect_receiver (`self.finalDotdamage`) (`self.finalDotNum`)))))