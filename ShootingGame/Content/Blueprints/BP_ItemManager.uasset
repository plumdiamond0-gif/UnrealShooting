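; BP_ItemManager is an item manager actor that applies a buff to the player when ItemApply is called with an item type.
; It searches the ItemDatas list in the Game Instance's ItemDataTable for entries of that type.
; Damage, attack speed and move speed buffs multiply the player's damage, shoot force and speed with no revert, while health buffs call GetHeal.
; It also prints the item type on each call.
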(event `ItemApply`
  (params (ItemType :type "/Game/Blueprints/EState/EState_Item Enum" :default "NewEnumerator0"))
  (bind _asbp_game_instance (cast `/Game/Blueprints/BP_GameInstance` (`GameplayStatics.GetGameInstance`)))
  (`KismetSystemLibrary.PrintString` (`|GetEnumeratorNameAsString` ItemType))
  (for _array_element (`/Game/Blueprints/DA/BP_ItemDataTable.ItemDatas` (`/Game/Blueprints/BP_GameInstance.ItemDataTable` _asbp_game_instance))
    (if (`|EnumEquality` (`.InItemType_23_0EFB35C64F4033E0B1E3B1A45CE1999A` (break `/Game/Blueprints/ST/ST_InItemData` _array_element)) ItemType)
      (bind _asbp_player (cast `/Game/Blueprints/Player/BP_Player` (`GameplayStatics.GetPlayerPawn` 0)))
      (switch `/Game/Blueprints/EState/EState_Item` ItemType
        (:`NewEnumerator0`
          (set `/Game/Blueprints/Player/BP_Player.PlayerDamage` (* (break `/Game/Blueprints/ST/ST_InItemData` _array_element) (`/Game/Blueprints/Player/BP_Player.PlayerDamage` _asbp_player)) _asbp_player))
        (:`NewEnumerator1`
          (`/Game/Blueprints/Player/BP_Player.GetHeal` _asbp_player (`.HealthBuff_12_131DCCC74D1F84BD5858A78281064D56` (break `/Game/Blueprints/ST/ST_InItemData` _array_element))))
        (:`NewEnumerator2`
          (set `/Game/Blueprints/Player/BP_Player.PlayerShootForce` (* (`/Game/Blueprints/Player/BP_Player.PlayerShootForce` _asbp_player) (`.AttackSpeedBuff_10_641AACB14458A8BE5C94E69D24D604EE` (break `/Game/Blueprints/ST/ST_InItemData` _array_element))) _asbp_player))
        (:`NewEnumerator3`
          (set `/Game/Blueprints/Player/BP_Player.PlayerSpeed` (* (`.MoveSpeedBuff_9_5F0E8EA54CA79BA92216779AE85BE127` (break `/Game/Blueprints/ST/ST_InItemData` _array_element)) (`/Game/Blueprints/Player/BP_Player.PlayerSpeed` _asbp_player)) _asbp_player))))))

(fn `UserConstructionScript`)