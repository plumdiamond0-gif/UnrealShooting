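; ObjectPool is a general-purpose actor pool that keeps spawned actors of one class for reuse.
; Initialize stores the class and pre-spawns actors into the PoolObjects array.
; Get pops the last pooled actor, or spawns a new one when the array is empty, and Return appends an actor back.
; The pool never changes an actor's visibility, collision or state on spawn, Get or Return.
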(event `Initialize`
  (params (actorClass :type "Actor Class Reference") (count :type Integer))
  (bind _output_get (set `self.Actor Class` actorClass))
  (for _ (range (+ count 1))
    (bind _returnvalue (`|SpawnActorFromClass` _output_get (`KismetMathLibrary.MakeTransform` (0.0 0.0 0.0)) "AlwaysSpawn" "MultiplyWithRoot" null null))
    (`KismetArrayLibrary.Array_Add` (`self.PoolObjects`) _returnvalue)))

(fn `Get`
  (returns (Obj :type "Actor Object Reference"))
  (bind _poolobjects (`self.PoolObjects`))
  (bind _returnvalue (`KismetArrayLibrary.Array_LastIndex` _poolobjects))
  (if (> (`KismetArrayLibrary.Array_Length` (`self.PoolObjects`)) 0)
    (set `self.poolObj` (`|GetArrayItem` _poolobjects _returnvalue))
    (`KismetArrayLibrary.Array_Remove` _poolobjects _returnvalue)
    (else
      (bind _returnvalue_2 (`|SpawnActorFromClass` (`self.Actor Class`) (`KismetMathLibrary.MakeTransform` (0.0 0.0 0.0)) "AlwaysSpawn" "MultiplyWithRoot" null null))
      (set `self.poolObj` _returnvalue_2)))
  (return (`self.poolObj`)))

(fn `Return`
  (params (returnedObj :type "Actor Object Reference"))
  (`KismetArrayLibrary.Array_Add` (`self.PoolObjects`) returnedObj))

(fn `UserConstructionScript`)