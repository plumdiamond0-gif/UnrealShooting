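; Player controller that manages UI panels, level setup and transitions, and post-reward upgrades for BP_Player.
; Level setup fades in and sets movement and attack permissions, adding the HUD in battle; level moves fade out before the GameInstance switches levels.
; The reward panel shows shuffled GameInstance table entries with random rolled values, applying the chosen one on close.
; A shared ShowPanel helper creates panels and switches to UI-only input.
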(event `self.ReceiveBeginPlay`
  (`EnhancedInputSubsystemInterface.AddMappingContext` (pcsubsystem `EnhancedInputLocalPlayerSubsystem` self) "/Game/Input/IMC_Player.IMC_Player" 0 (struct)))

(event `CloseRewardPanel`
  (params (Num :type Integer))
  (`Widget.RemoveFromParent` (stale `ShowRewardPanel` _returnvalue))
  (bind _asbp_player (cast `/Game/Blueprints/Player/BP_Player` (`GameplayStatics.GetPlayerCharacter` 0)))
  (`/Game/Blueprints/Player/BP_Player.ApplyReward` _asbp_player (`.Type_2_63C421704075EF395D1BD69B7E563BE0` (break `/Game/Blueprints/ST/ST_RewardData` (`|GetArrayItem` (`self.RewardDatas`) Num))) (`|GetArrayItem` (`self.RanVals`) Num))
  (`/Game/Blueprints/Player/BP_Player.CallReward` _asbp_player)
  (bind _asbp_player_2 (cast `/Game/Blueprints/Player/BP_Player` (`GameplayStatics.GetPlayerPawn` 0)))
  (set `/Game/Blueprints/AC/AC_Move.CanMove` true (`/Game/Blueprints/Player/BP_Player.AC_Move` _asbp_player_2))
  (`WidgetBlueprintLibrary.SetInputMode_GameOnly` self)
  (set `self.bShowMouseCursor` false))

(event `ShowRewardPanel`
  (bind _returnvalue (`|CreateWidget` "/Game/Blueprints/Player/Panel/Reward/WBP_RewardPanel.WBP_RewardPanel_C"))
  (`UserWidget.AddToViewport` _returnvalue 0)
  (`self.GetRandomVal` _returnvalue)
  (`/Game/Blueprints/Player/Panel/WBP_PanelBase.OpenPanel` _returnvalue)
  (add `/Game/Blueprints/Player/Panel/Reward/WBP_RewardPanel.ED_LastProcess` _returnvalue (delegate `CloseRewardPanel`)))

(event `LevelSetUp`
  (params (Level :type "/Game/Blueprints/EState/EState_Level Enum" :default "NewEnumerator0"))
  (switch `/Game/Blueprints/EState/EState_Level` Level
    (:`NewEnumerator0`
      (bind _newparam (`self.ShowPanel` "/Game/Blueprints/Player/Panel/WBP_FadePanel.WBP_FadePanel_C"))
      (bind _aswbp_fade_panel (cast `/Game/Blueprints/Player/Panel/WBP_FadePanel` _newparam))
      (`/Game/Blueprints/Player/Panel/WBP_FadePanel.PanelFade` _aswbp_fade_panel true)
      (bind _asbp_player (cast `/Game/Blueprints/Player/BP_Player` (`GameplayStatics.GetPlayerPawn` 0)))
      (set `/Game/Blueprints/Player/BP_Player.CanAttack` false _asbp_player)
      (set `/Game/Blueprints/AC/AC_Move.CanMove` true (`/Game/Blueprints/Player/BP_Player.AC_Move` _asbp_player))
      (`WidgetBlueprintLibrary.SetInputMode_GameOnly` self))
    (:`NewEnumerator2`
      (bind _newparam_2 (`self.ShowPanel` "/Game/Blueprints/Player/Panel/WBP_FadePanel.WBP_FadePanel_C"))
      (bind _aswbp_fade_panel_2 (cast `/Game/Blueprints/Player/Panel/WBP_FadePanel` _newparam_2))
      (`/Game/Blueprints/Player/Panel/WBP_FadePanel.PanelFade` _aswbp_fade_panel_2 true)
      (`KismetSystemLibrary.Delay` 1.0)
      (`self.ShowPanel` "/Game/Blueprints/Player/Panel/HUD/WBP_PlayerHUD.WBP_PlayerHUD_C")
      (bind _asbp_player_2 (cast `/Game/Blueprints/Player/BP_Player` (`GameplayStatics.GetPlayerPawn` 0)))
      (set `/Game/Blueprints/AC/AC_Move.CanMove` true (`/Game/Blueprints/Player/BP_Player.AC_Move` _asbp_player_2))
      (`WidgetBlueprintLibrary.SetInputMode_GameOnly` self)
      (set `/Game/Blueprints/Player/BP_Player.CanAttack` true _asbp_player_2))))

(event `MoveLevel`
  (params (Type :type "/Game/Blueprints/EState/EState_Level Enum" :default "NewEnumerator0"))
  (bind _newparam (`self.ShowPanel` "/Game/Blueprints/Player/Panel/WBP_FadePanel.WBP_FadePanel_C"))
  (bind _aswbp_fade_panel (cast `/Game/Blueprints/Player/Panel/WBP_FadePanel` _newparam))
  (`/Game/Blueprints/Player/Panel/WBP_FadePanel.PanelFade` _aswbp_fade_panel false)
  (`KismetSystemLibrary.Delay` 1.0)
  (bind _asbp_game_instance (cast `/Game/Blueprints/BP_GameInstance` (`GameplayStatics.GetGameInstance`)))
  (`/Game/Blueprints/BP_GameInstance.MoveLevel` _asbp_game_instance Type))

(fn `GetRandomVal`
  (params (RewardPanel :type "/Game/Blueprints/Player/Panel/Reward/WBP_RewardPanel Object Reference"))
  (bind _ranval (`self.RanVal`))
  (bind _asbp_game_instance (cast `/Game/Blueprints/BP_GameInstance` (`GameplayStatics.GetGameInstance`)))
  (bind _output_get (set `self.RewardDatas` (`/Game/Blueprints/DA/BP_RewardDataTable.RewardDatas` (`/Game/Blueprints/BP_GameInstance.RewardDataTable` _asbp_game_instance))))
  (`KismetArrayLibrary.Array_Shuffle` _output_get)
  (`KismetArrayLibrary.Array_Clear` (`self.RanVals`))
  (for (_array_element _array_index) (`/Game/Blueprints/Player/Panel/Reward/WBP_RewardPanel.RewardCells` RewardPanel)
    (set `/Game/Blueprints/Player/Panel/Reward/WBP_RewardCell.Num` _array_index _array_element)
    (bind (_output_type _output_minval _output_maxval _output_texture _output_isadd) (break `/Game/Blueprints/ST/ST_RewardData` (`|GetArrayItem` (`self.RewardDatas`) _array_index)))
    (if _output_isadd
      (set `self.RanVal` (`KismetMathLibrary.Conv_IntToDouble` (`KismetMathLibrary.Round` (`KismetMathLibrary.RandomFloatInRange` _output_minval _output_maxval))))
      (else
        (set `self.RanVal` (/ (`KismetMathLibrary.Round` (* (`KismetMathLibrary.RandomFloatInRange` _output_minval _output_maxval) 10.0)) 10))))
    (`/Game/Blueprints/Player/Panel/Reward/WBP_RewardCell.SetInfo` _array_element _output_type _ranval _output_texture _output_isadd)
    (`KismetArrayLibrary.Array_Add` (`self.RanVals`) _ranval)))

(fn `RemovePanel`
  (params (Widget :type "Widget Object Reference"))
  (`/Engine/EditorBlueprintResources/StandardMacros.IsValid` Widget
    (:`Is Valid`
      (`Widget.RemoveFromParent` Widget))
    (:`Is Not Valid`
      _))
  (`WidgetBlueprintLibrary.SetInputMode_GameOnly` self)
  (set `self.bShowMouseCursor` false))

(fn `ShowPanel`
  (params (Class :type "Object Class Reference"))
  (returns (NewParam :type "Widget Object Reference"))
  (bind _aswbp_panel_base (castclass `/Game/Blueprints/Player/Panel/WBP_PanelBase` Class))
  (bind _returnvalue (`|CreateWidget` _aswbp_panel_base))
  (`UserWidget.AddToViewport` _returnvalue 0)
  (`WidgetBlueprintLibrary.SetInputMode_UIOnlyEx` self _returnvalue "LockAlways")
  (set `self.bShowMouseCursor` true)
  (`/Game/Blueprints/Player/Panel/WBP_PanelBase.OpenPanel` _returnvalue)
  (return _returnvalue))

(fn `UserConstructionScript`)