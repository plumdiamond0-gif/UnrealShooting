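; BP_Bullet is a reusable player projectile that damages BP_Enemy actors on overlap.
; ActivateBullet stores damage, effects and origin, then shows the bullet, enables query collision and sets its velocity.
; On an enemy hit it calls the HealthComponent's GetDamage, deactivates itself by hiding and stopping rather than being destroyed, then applies each bullet effect.
; A Tick max-distance cutoff exists but is disabled by a constant false condition.
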(event `self.ReceiveBeginPlay`)

(event `self.ReceiveTick`
  (params (DeltaSeconds :type "Float (single-precision)"))
  (if (and (> (`KismetMathLibrary.Vector_Distance` (`self.OriPos`) (`self.K2_GetActorLocation`)) (`self.MaxDist`)) false)
    (`self.SetActorHiddenInGame` true)
    (set `MovementComponent.Velocity` (0.0 0.0 0.0) (`self.ProjectileMovement`))))

(event `DeActivateBullet`
  ; 탄환 비활성화
  (`PrimitiveComponent.SetCollisionEnabled` (`self.Sphere`) "NoCollision")
  (`ActorComponent.SetActive` (`self.ProjectileMovement`) false false)
  (`self.SetActorHiddenInGame` true)
  (set `MovementComponent.Velocity` (0.0 0.0 0.0) (`self.ProjectileMovement`)))

(event `ActivateBullet`
  (params (Velocity :type "Vector Structure") (Pos :type "Vector Structure") (FinalDamage :type "Float (double-precision)") (BulletEffects :type "Array of /Game/Blueprints/DA/Effect/BP_BulletEffect Object Reference"))
  ; 탄환 활성화
  (set `self.Bullet Effects` BulletEffects)
  (set `self.Damage` FinalDamage)
  (`ActorComponent.SetActive` (`self.ProjectileMovement`) true false)
  (set `self.OriPos` Pos)
  (`self.SetActorHiddenInGame` false)
  (`PrimitiveComponent.SetCollisionEnabled` (`self.Sphere`) "QueryOnly")
  (set `MovementComponent.Velocity` Velocity (`self.ProjectileMovement`)))

(event `self.Sphere.OnComponentBeginOverlap`
  (params (OverlappedComponent :type "PrimitiveComponent Object Reference") (OtherActor :type "Actor Object Reference") (OtherComp :type "PrimitiveComponent Object Reference") (OtherBodyIndex :type Integer) (bFromSweep :type Boolean) (SweepResult :type "HitResult Structure (by ref)"))
  ; 적에게 닿았을 시
  (bind _asbp_enemy (cast `/Game/Blueprints/Enemy/BP_Enemy` OtherActor))
  (`/Game/Blueprints/AC/AC_Health.GetDamage` (`/Game/Blueprints/Enemy/BP_Enemy.HealthComponent` _asbp_enemy) (`self.Damage`))
  (`self.DeActivateBullet`)
  (for _array_element (`self.Bullet Effects`)
    (`/Game/Blueprints/BPI/BPI_BulletEffect.ApplyEffect` _array_element null 1.0)))

(fn `UserConstructionScript`)